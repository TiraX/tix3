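; BP_TiXExporter is an editor-facing actor that exports the current level or a chosen static mesh through the TiX exporter functions.
; ExportLevel and ExportStaticMesh each first run ApplySettings, then call the matching export function.
; ApplySettings pushes the actor's variables for material ignoring, tile size, vertex position scale and export path into the exporter.
; The BeginPlay, overlap and Tick events and the construction script are empty.
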(fn `ApplySettings`
  (`|ExecutionSequence`
    (:`then_0`
      (`TiXExporterBPLibrary.SetIgnoreMaterial` (`self.IgnoreMaterial`)))
    (:`then_1`
      (`TiXExporterBPLibrary.SetTileSize` (`self.TileSize`)))
    (:`then_2`
      (`TiXExporterBPLibrary.SetMeshVertexPositionScale` (`self.PositionScale`)))
    (:`then_3`
      (`TiXExporterBPLibrary.SetExportPath` (`.Path` (break `DirectoryPath` (`self.ExportPath`)))))))

(fn `ExportLevel`
  (`|ExecutionSequence`
    (:`then_0`
      (`self.ApplySettings`))
    (:`then_1`
      (`TiXExporterBPLibrary.ExportCurrentLevel` self))))

(fn `ExportStaticMesh`
  (`|ExecutionSequence`
    (:`then_0`
      (`self.ApplySettings`))
    (:`then_1`
      (`TiXExporterBPLibrary.ExportStaticMesh` (`self.Static Mesh`)))))

(fn `UserConstructionScript`)